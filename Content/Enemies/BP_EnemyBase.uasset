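; Base enemy actor that flies straight along its spawn-time forward vector and fires at a fixed interval.
; Tick moves it without sweep and runs a timer that spawns Ammo at FirePoint, matching the enemy's rotation.
; Capsule overlap with a Player-tagged actor calls the OnEnemyDestroy dispatcher, whose bound event destroys it after a short delay, and notifies BP_00_GameMode.
; An unconnected BP_PlayerAmmo cast into that death path never runs.
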(event `self.ReceiveBeginPlay`
  ;[1 1 1] Enemy movement and destroy
  (set `self.MovementVector` (`self.GetActorForwardVector`))
  (add `self.OnEnemyDestroy` (delegate `DestroyedEvent`)))

(event `DestroyedEvent`
  ;[1 1 1] Enemy movement and destroy
  (`KismetSystemLibrary.Delay` 0.1)
  (`self.K2_DestroyActor`))

(event `self.CapsuleComponent.OnComponentBeginOverlap`
  (params (OverlappedComponent :type "PrimitiveComponent Object Reference") (OtherActor :type "Actor Object Reference") (OtherComp :type "PrimitiveComponent Object Reference") (OtherBodyIndex :type Integer) (bFromSweep :type Boolean) (SweepResult :type "HitResult Structure (by ref)"))
  ;[1 1 1] Enemy Destroyed logic
  (if (`KismetArrayLibrary.Array_Contains` (`Actor.Tags` OtherActor) "Player")
    (`self.OnEnemyDestroy`)
    (bind _asbp_00_game_mode (cast `/Game/Player/BP_00_GameMode` (`GameplayStatics.GetGameMode`)))
    (`/Game/Player/BP_00_GameMode.EnemyDestroyed` _asbp_00_game_mode)))

(event `self.ReceiveTick`
  (params (DeltaSeconds :type "Float (single-precision)"))
  ;[1 1 1] Shooting logic
  (`self.Move` DeltaSeconds)
  (bind _output_get (set `self.ShotCurrentTime` (+ DeltaSeconds (`self.ShotCurrentTime`))))
  (if (> _output_get (`self.FireDelay`))
    (set `self.ShotCurrentTime` 0.0)
    (`self.Do Fire`)))

(fn `Do Fire`
  (bind _returnvalue (`|SpawnActorFromClass` (`self.Ammo`) (`SceneComponent.K2_GetComponentToWorld` (`self.FirePoint`)) "Undefined" "MultiplyWithRoot" null null))
  (`self.K2_SetActorRotation` _returnvalue (`self.K2_GetActorRotation`) false))

(fn `Move`
  (params (`Delta Time` :type "Float (double-precision)"))
  (`self.K2_SetActorLocation` (+ (`self.K2_GetActorLocation`) (* (* `Delta Time` (`self.Speed`)) (`self.MovementVector`)))))

(fn `UserConstructionScript`)